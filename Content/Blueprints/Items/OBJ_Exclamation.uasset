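; OBJ_Exclamation is a world marker actor that shows a text label, such as an exclamation, when the player is nearby.
; Each tick it compares its distance to the player character against SeeableDistance, showing or hiding the TextRender component accordingly.
; While visible, the text rotates to face the player using a look-at rotation.
; The construction script applies the configurable Text variable to the TextRender.
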(event `self.ReceiveTick`
  (params (DeltaSeconds :type "Float (single-precision)"))
  (bind _returnvalue (`self.K2_GetActorLocation`))
  (bind _textrender (`self.TextRender`))
  (bind _returnvalue_2 (`self.K2_GetActorLocation` (`GameplayStatics.GetPlayerCharacter` 0)))
  (if (< (`KismetMathLibrary.VSize` (- _returnvalue_2 _returnvalue)) (`self.See-able Distance`))
    (`SceneComponent.SetVisibility` _textrender true false)
    (`SceneComponent.K2_SetWorldRotation` (`self.TextRender`) (`KismetMathLibrary.FindLookAtRotation` _returnvalue _returnvalue_2) false false)
    (else
      (`SceneComponent.SetVisibility` _textrender false false))))

(fn `UserConstructionScript`
  (`TextRenderComponent.K2_SetText` (`self.TextRender`) (`self.Text`)))