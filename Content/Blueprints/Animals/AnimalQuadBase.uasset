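; Base Blueprint for a quadruped animal with its own velocity-based movement.
; AddMovementInput adds normalized direction times walk speed to Velocity, which Tick's Move applies as a swept, rotation-relative offset, dividing horizontal velocity by ground friction when grounded.
; Capsule-radius line traces against WorldStatic provide ground check, floor normal and height; the first two trace toward +Z.
; No gravity is applied here, and floor normal and height go unused.
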(event `self.ReceiveTick`
  (params (DeltaSeconds :type "Float (single-precision)"))
  (`self.Move`))

(fn `Add Movement Input`
  (params (Direction :type "Vector Structure"))
  (set `self.Velocity` (+ (* (`KismetMathLibrary.Normal` Direction) (`self.Max Walk Speed`)) (`self.Velocity`))))

(fn `Check On Ground`
  (returns (isOnGround :type Boolean))
  (bind _returnvalue (`self.K2_GetActorLocation`))
  (bind (_outhit _returnvalue_2) (`KismetSystemLibrary.LineTraceSingleForObjects` _returnvalue (+ _returnvalue (`KismetMathLibrary.MakeVector` 0.0 0.0 (+ (`CapsuleComponent.CapsuleRadius` (`self.Capsule`)) 5.0))) (`|MakeArray` "ObjectTypeQuery1" :!type "EObjectTypeQuery Enum") true))
  (return _returnvalue_2))

(fn `Get Floor Normal`
  (returns (`Floor Normal` :type "Vector Structure"))
  (bind _returnvalue (`self.K2_GetActorLocation`))
  (bind (_outhit _returnvalue_2) (`KismetSystemLibrary.LineTraceSingleForObjects` _returnvalue (+ _returnvalue (`KismetMathLibrary.MakeVector` 0.0 0.0 (+ (`CapsuleComponent.CapsuleRadius` (`self.Capsule`)) 10.0))) (`|MakeArray` "ObjectTypeQuery1" :!type "EObjectTypeQuery Enum") true))
  (if _returnvalue_2
    (return (`.Normal` (`GameplayStatics.BreakHitResult` _outhit)))
    (else
      (return (0.0 0.0 0.0)))))

(fn `Height From Ground`
  (returns (`Height From Ground` :type "Float (double-precision)"))
  (bind _returnvalue (`self.K2_GetActorLocation`))
  (bind _capsuleradius (`CapsuleComponent.CapsuleRadius` (`self.Capsule`)))
  (bind _outhit (`KismetSystemLibrary.LineTraceSingleForObjects` (- _returnvalue (* (`self.GetActorUpVector`) (* _capsuleradius -1.0))) (- _returnvalue (`KismetMathLibrary.MakeVector` 0.0 0.0 (+ _capsuleradius 10000.0))) (`|MakeArray` "ObjectTypeQuery1" :!type "EObjectTypeQuery Enum") true))
  (return (`.Distance` (`GameplayStatics.BreakHitResult` _outhit))))

(fn `Move`
  (bind _velocity (`self.Velocity`))
  (bind _ground_friction (`self.Ground Friction`))
  (`self.K2_AddActorWorldOffset` (* (`KismetMathLibrary.GreaterGreater_VectorRotator` _velocity (`self.K2_GetActorRotation`)) (`GameplayStatics.GetWorldDeltaSeconds`)) true)
  (bind _isonground (`self.Check On Ground`))
  (if _isonground
    (set `self.Velocity` (/ _velocity (`KismetMathLibrary.MakeVector` _ground_friction _ground_friction 1.0)))))

(fn `UserConstructionScript`
  (`parent.UserConstructionScript`))